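; BP_Frac is a breakable Chaos object that awards score when smashed in the roller game, optionally counting as a pin.
; It keeps the FRAC component's tick off until an actor overlaps, then destroys the trigger, re-enables tick and restores the starting transform.
; Each break event adds mass-scaled points through RollerGameMode.
; The first break also adds pin score if flagged and fires particles at the break location using its local-space velocity.
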(event Custom|OnChaosBreakEvent_Event_0
  (params (BreakEvent :type Chaos%20Break%20Event%20Structure%20%28by%20ref%29))
  (bind _breakeffect (Variables|Default|GetBreakEffect))
  (Development|PrintString (Utilities|String|ToString(Float) (.mass BreakEvent)))
  ;[1 1 1] Add points based on mass of broken pieces
  (bind _asroller_game_mode (Utilities|Casting|CastToRollerGameMode (Game|GetGameMode)))
  (Default|ADDSCOREPOINTS _asroller_game_mode (* (.mass BreakEvent) (Variables|Default|GetPointMultiplier)))
  ;[1 1 1] Continue if this is the first break
  (if (not (Variables|Default|GetAlreadyBroken))
    (Variables|Default|SetAlreadyBroken true)
    ;[1 1 1] Add pin score if this is a pin
    (if (Variables|Default|GetIsPin)
      (Default|ADDPINSCORE _asroller_game_mode 1))
    ;[1 1 1] Trigger particles
    (Effects|Components|ParticleSystem|SetVectorParameter _breakeffect "BreakVelocity" (Math|Transform|InverseTransformDirection (Transformation|GetActorTransform) (.velocity BreakEvent)))
    (Transformation|SetWorldLocation _breakeffect (.location BreakEvent) false false)
    (Components|Activation|Activate _breakeffect false)))

(event EventBeginPlay
  (Variables|Default|SetOriginalPos (Transformation|GetWorldTransform (Variables|Default|GetFRAC)))
  ;[1 1 1] Make object sleep
  (Components|Tick|SetComponentTickEnabled (Variables|Default|GetFRAC) false)
  (EventDispatchers|AssignOnChaosBreakEvent (Variables|Default|GetFRAC) (delegate Custom|OnChaosBreakEvent_Event_0)))

(event Collision|EventActorBeginOverlap
  (params (OtherActor :type Actor%20Object%20Reference))
  (Components|DestroyComponent (Variables|Default|GetTrigger))
  (Components|Tick|SetComponentTickEnabled (Variables|Default|GetFRAC) true)
  (Transformation|SetWorldTransform (Variables|Default|GetFRAC) (Variables|Default|GetOriginalPos) false true))

(fn ConstructionScript)